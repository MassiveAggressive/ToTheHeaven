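; BP_InteractBase is an interactable actor, named as a base, that shows an interaction key prompt while the player is in range.
; Its box trigger, sized from BoxExtent in the construction script, creates a W_InteractKey widget and adds it to the viewport when BP_Player begins overlapping.
; The prompt is removed when the overlap ends or Interact fires, which does nothing else here.
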(event OnComponentBeginOverlap(Box)
  (params (OverlappedComponent :type Primitive%20Component%20Object%20Reference) (OtherActor :type Actor%20Object%20Reference) (OtherComp :type Primitive%20Component%20Object%20Reference) (OtherBodyIndex :type Integer) (bFromSweep :type Boolean) (SweepResult :type Hit%20Result%20Structure%20%28by%20ref%29))
  (Utilities|Casting|CastToBP_Player OtherActor)
  (bind _returnvalue (UserInterface|CreateWidget "/Game/Blueprints/Puzzle/Widget/W_InteractKey.W_InteractKey_C"))
  (bind _output_get (Variables|Default|SetW_InteractWidget _returnvalue))
  (UserInterface|Viewport|AddtoViewport _output_get 0))

(event OnComponentEndOverlap(Box)
  (params (OverlappedComponent :type Primitive%20Component%20Object%20Reference) (OtherActor :type Actor%20Object%20Reference) (OtherComp :type Primitive%20Component%20Object%20Reference) (OtherBodyIndex :type Integer))
  (Utilities|Casting|CastToBP_Player OtherActor)
  (Widget|RemovefromParent (Variables|Default|GetW_InteractWidget)))

(event EventInteract
  (Widget|RemovefromParent (Variables|Default|GetW_InteractWidget)))

(fn ConstructionScript
  (Components|Box|SetBoxExtent (Variables|Default|GetBox) (Variables|Default|GetBoxExtent) true))