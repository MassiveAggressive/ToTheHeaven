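; Puzzle condition that completes when an item named "Key" is added to the player's inventory.
; On BeginPlay it gets player controller 0 as BP_InGamePlayerController and binds to the item-added event of its ACInventoryEquipment component.
; The CheckKey handler compares the item's name to a hardcoded literal and fires ConditionComplete on a match.
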(event Custom|CheckKey
  (params (Item :type S%20Item%20Structure))
  (if (Utilities|Enum|Equal(Enum) (Utilities|Struct|BreakS_Item Item) (Utilities|Text|MakeLiteralText "Key"))
    (Default|CallConditionComplete)))

(event EventBeginPlay
  (bind _asbp_in_game_player_controller (Utilities|Casting|CastToBP_InGamePlayerController (Game|GetPlayerController 0)))
  (EventDispatchers|BindEventtoItemAddedtoInventory (Variables|/Game/Blueprints/Player/BP_InGamePlayerController.BP_InGamePlayerController_C|GetAC_InventoryEquipment _asbp_in_game_player_controller) (EventDispatchers|CreateEvent :!event Custom|CheckKey)))

(fn ConstructionScript
  (|CallParentFunction))