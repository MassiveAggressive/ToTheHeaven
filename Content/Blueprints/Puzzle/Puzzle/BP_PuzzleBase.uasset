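; Base puzzle actor that tracks a set of conditions and signals when the puzzle is solved.
; On Interact it runs the parent behavior, spawns an actor for each entry in ConditionClasses, stores it and binds to its ConditionComplete dispatcher.
; Each completion increments a counter, and the PuzzleSolved dispatcher fires once the count reaches the number of condition classes.
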(event Custom|ConditionComplete
  (bind _result (Math|Integer|IncrementInt (Variables|Default|GetCompletedConditionsNum))
    (:%20%20
      (if (>= _result (Utilities|Array|Length (Variables|Default|GetConditionClasses)))
        (Default|CallPuzzleSolved)))))

(event EventInteract
  (|CallParentFunction)
  (for _array_element (Variables|Default|GetConditionClasses)
    (bind _returnvalue (Game|SpawnActorfromClass _array_element (Math|Transform|MakeTransform "0, 0, 0" "0, 0, 0" "1,1,1") "AlwaysSpawn" 0 0))
    (Utilities|Array|Add (Variables|Default|GetConditions) _returnvalue)
    (EventDispatchers|BindEventtoConditionComplete _returnvalue (EventDispatchers|CreateEvent :!event Custom|ConditionComplete))))

(fn ConstructionScript)