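; Blueprint function library of global helpers for floor-based travel and game progression state.
; Floor index, previous floor, travel availability, open state and condition calls all forward to BP_GameInstance, which holds that state.
; TravelToFloor records the new floor index in the game instance, then hands the move to BP_InGameGameMode.
; Each function casts to its target class and does nothing if the cast fails.
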(fn TraveltoFloor
  (params (FloorIndex :type Integer))
  (bind _asbp_in_game_game_mode (Utilities|Casting|CastToBP_InGameGameMode (Game|GetGameMode)))
  (CallFunction|SetCurrentFloorIndex FloorIndex)
  (Default|TraveltoFloor _asbp_in_game_game_mode FloorIndex))

(fn GetCurrentFloorIndex
  (bind _asbp_game_instance (Utilities|Casting|CastToBP_GameInstance (Game|GetGameInstance)))
  (return (Default|GetCurrentFloorIndex _asbp_game_instance)))

(fn SetCurrentFloorIndex
  (params (FloorIndex :type Integer))
  (bind _asbp_game_instance (Utilities|Casting|CastToBP_GameInstance (Game|GetGameInstance)))
  (Default|SetCurrentFloorIndex _asbp_game_instance FloorIndex))

(fn GetPreviousFloorIndex
  (bind _asbp_game_instance (Utilities|Casting|CastToBP_GameInstance (Game|GetGameInstance)))
  (return (Default|GetPreviousFloorIndex _asbp_game_instance)))

(fn GetIsAvailableTraveltoFloor
  (params (FloorIndex :type Integer))
  (bind _asbp_game_instance (Utilities|Casting|CastToBP_GameInstance (Game|GetGameInstance)))
  (return (Default|GetIsAvailableTraveltoFloor _asbp_game_instance FloorIndex)))

(fn AddCondition
  (params (NewCondition :type BP%20Condition%20Base%20Class%20Reference))
  (bind _asbp_game_instance (Utilities|Casting|CastToBP_GameInstance (Game|GetGameInstance)))
  (Default|AddCondition _asbp_game_instance NewCondition))

(fn SetFloorIsOpen
  (params (FloorIndex :type Integer) (IsOpen :type Boolean))
  (bind _asbp_game_instance (Utilities|Casting|CastToBP_GameInstance (Game|GetGameInstance)))
  (Default|SetFloorIsOpen _asbp_game_instance FloorIndex IsOpen))