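; BP_Floor is a floor volume that is either locked or unlocked and detects when the player enters it.
; Its Box, sized from BoxExtent in the construction script, blocks all channels when Locked and overlaps them when Unlocked.
; The initial state is applied on BeginPlay, and completion of the Condition component unlocks the floor.
; A BP_Player beginning overlap with the Box triggers CallPlayerDetected with the FloorIndex.
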(event OnComponentBeginOverlap(Box)
  (params (OverlappedComponent :type Primitive%20Component%20Object%20Reference) (OtherActor :type Actor%20Object%20Reference) (OtherComp :type Primitive%20Component%20Object%20Reference) (OtherBodyIndex :type Integer) (bFromSweep :type Boolean) (SweepResult :type Hit%20Result%20Structure%20%28by%20ref%29))
  (Utilities|Casting|CastToBP_Player OtherActor)
  (Default|CallPlayerDetected (Variables|Default|GetFloorIndex)))

(event ConditionComplete(Condition)
  (CallFunction|SetFloorStatue "NewEnumerator1"))

(event EventBeginPlay
  (CallFunction|SetFloorStatue (Variables|Default|GetFloorStatue)))

(fn ConstructionScript
  (Components|Box|SetBoxExtent (Variables|Default|GetBox) (Variables|Default|GetBoxExtent) true))

(fn SetFloorStatue
  (params (Statue :type E_FloorStatue%20Enum :default "NewEnumerator0"))
  (bind _box (Variables|Default|GetBox))
  (bind _output_get (Variables|Default|SetFloorStatue Statue))
  (switch Utilities|FlowControl|Switch|SwitchonE_FloorStatue _output_get
    (:NewEnumerator0
      (Collision|SetCollisionResponsetoAllChannels _box "ECR_Block"))
    (:NewEnumerator1
      (Collision|SetCollisionResponsetoAllChannels _box "ECR_Overlap"))))