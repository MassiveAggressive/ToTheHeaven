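; Base player controller that toggles on-screen widgets through a map of input keys to widgets.
; AddWidget registers a widget under a key, adds it to the viewport and starts it collapsed.
; Any mapped key press shows its widget after collapsing all others, or collapses it if already visible.
; A separate Tab handler toggles its widget without collapsing the others or checking that the key is mapped.
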(event EventAddWidget
  (params (Key :type Key%20Structure :default "None") (Widget :type User%20Widget%20Object%20Reference))
  (Utilities|Map|Add (Variables|Default|GetWidgets) Key Widget)
  (UserInterface|Viewport|AddtoViewport Widget 0)
  (Widget|SetVisibility Widget "Collapsed"))

(event Input|KeyboardEvents|AnyKey
  (params (Key :type Key%20Structure :default "None"))
  (bind _widgets (Variables|Default|GetWidgets))
  (bind (_value _returnvalue) (Utilities|Map|Find _widgets Key))
  (:Pressed
    (if _returnvalue
      (bind _output_get (Variables|Default|SetPressedWidget _value))
      (if (not (Widget|IsVisible _output_get))
        (bind _keys (Utilities|Map|Keys (Variables|Default|GetWidgets)))
        (for _array_element _keys
          (Widget|SetVisibility (.Value (Utilities|Map|Find (Variables|Default|GetWidgets) _array_element)) "Collapsed"))
        (Widget|SetVisibility (Variables|Default|GetPressedWidget) "Visible")
        (else
          (Widget|SetVisibility (Variables|Default|GetPressedWidget) "Collapsed"))))))

(event Input|KeyboardEvents|Tab
  (params (Key :type Key%20Structure :default "None"))
  (bind _widgets (Variables|Default|GetWidgets))
  (bind _value (Utilities|Map|Find _widgets Key))
  (:Pressed
    (if (Widget|IsVisible _value)
      (Widget|SetVisibility _value "Collapsed")
      (else
        (Widget|SetVisibility _value "Visible")))))

(fn ConstructionScript)